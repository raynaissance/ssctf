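; SuperSpeedBoundingBox is an actor that stretches a collision box along the path of a super-speeding owner and ends the ability on overlap.
; Construction records the owner's ground-plane position as the start point.
; While following, Tick centers the box between start and owner, rotates it along that line and scales its length to the distance.
; On the server, overlapping another actor calls DoSuperSpeedEnd on the owning MyCharacter and destroys the box.
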(event `self.ReceiveTick`
  (params (DeltaSeconds :type "Float (single-precision)"))
  (bind _startpoint (`self.StartPoint`))
  (bind _returnvalue (`KismetMathLibrary.MakeVector` (.x (`self.K2_GetActorLocation` (`self.MyOwner`))) (.y (`self.K2_GetActorLocation` (`self.MyOwner`)))))
  (bind _returnvalue_2 (- _returnvalue _startpoint))
  (if (`self.isFollowingPlayer`)
    (`self.K2_SetActorLocation` (+ (/ _returnvalue_2 2.0) _startpoint))
    (`self.SetActorRotation` (`KismetMathLibrary.FindLookAtRotation` _startpoint _returnvalue))
    (`self.SetActorScale3D` (`KismetMathLibrary.MakeVector` (/ (`KismetMathLibrary.VSize` _returnvalue_2) 256.0) (.y (`self.GetActorScale3D`)) (.z (`self.GetActorScale3D`))))))

(event `self.BoundingBox.OnComponentBeginOverlap`
  (params (OtherActor :type "Actor Object Reference") (OtherComp :type "PrimitiveComponent Object Reference") (OtherBodyIndex :type Integer) (bFromSweep :type Boolean) (SweepResult :type "EngineTypes.HitResult Structure (by ref)"))
  (`/Engine/EditorBlueprintResources/ActorMacros.Switch Has Authority`
    (:`Authority`
      (if (!= OtherActor self)
        (bind _asmycharacter_c (cast `/Game/Blueprints/MyCharacter` (`self.MyOwner`)))
        (`/Game/Blueprints/MyCharacter.doSuperSpeedEnd` _asmycharacter_c)
        (`self.K2_DestroyActor`)))))

(fn `OnRep_isFollowingPlayer`)

(fn `UserConstructionScript`
  (bind _returnvalue (`KismetMathLibrary.MakeVector` (.x (`self.K2_GetActorLocation` (`self.MyOwner`))) (.y (`self.K2_GetActorLocation` (`self.MyOwner`)))))
  (`self.K2_SetActorLocation` _returnvalue)
  (set `self.StartPoint` _returnvalue))