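; BaseArea is a team base zone that scores rounds in a capture-the-flag mode.
; Server-only overlap events on BaseBox track whether the flag matching its TeamIndex is inside.
; If another team's flag enters while the home flag is present, it calls WinRound on the entering flag's Team reference, prints that score and resets that flag.
; This check runs only on entry, not when the home flag returns.
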(event `self.BaseBox.OnComponentBeginOverlap`
  (params (OtherActor :type "Actor Object Reference") (OtherComp :type "PrimitiveComponent Object Reference") (OtherBodyIndex :type Integer) (bFromSweep :type Boolean) (SweepResult :type "EngineTypes.HitResult Structure (by ref)"))
  (`/Engine/EditorBlueprintResources/ActorMacros.Switch Has Authority`
    (:`Authority`
      (bind _asflag_c (cast `/Game/Blueprints/Flag` OtherActor))
      (if (== (`/Game/Blueprints/Flag.TeamIndex` _asflag_c) (`self.TeamIndex`))
        (set `self.doesTeamFlagExistInBase` true)
        (elif (`self.doesTeamFlagExistInBase`)
          (bind _team (`/Game/Blueprints/Flag.Team` _asflag_c))
          (`/Game/Blueprints/Blueprints/team.winRound` _team)
          (`KismetSystemLibrary.PrintString` (`KismetStringLibrary.Concat_StrStr` "Score: " (`KismetStringLibrary.Conv_IntToString` (`/Game/Blueprints/Blueprints/team.Score` _team))))
          (`/Game/Blueprints/Flag.ResetWhenWin` _asflag_c))))))

(event `self.BaseBox.OnComponentEndOverlap`
  (params (OtherActor :type "Actor Object Reference") (OtherComp :type "PrimitiveComponent Object Reference") (OtherBodyIndex :type Integer))
  (`/Engine/EditorBlueprintResources/ActorMacros.Switch Has Authority`
    (:`Authority`
      (bind _asflag_c (cast `/Game/Blueprints/Flag` OtherActor))
      (if (== (`/Game/Blueprints/Flag.TeamIndex` _asflag_c) (`self.TeamIndex`))
        (set `self.doesTeamFlagExistInBase` false)))))

(fn `UserConstructionScript`)