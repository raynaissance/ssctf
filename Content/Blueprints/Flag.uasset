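; Capture-the-flag style flag actor that characters pick up by overlapping its mesh and carry until it is reset.
; On the server, an overlap with an eligible MyCharacter disables further pickup, attaches the flag to that character and sets its CarryingFlag reference.
; Reset, also authority-only, re-enables pickup, clears the carrier through ResetFlag, detaches and returns the flag to the location cached in the construction script.
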(event `self.StaticMesh1.OnComponentBeginOverlap`
  (params (OtherActor :type "Actor Object Reference") (OtherComp :type "PrimitiveComponent Object Reference") (OtherBodyIndex :type Integer) (bFromSweep :type Boolean) (SweepResult :type "EngineTypes.HitResult Structure (by ref)"))
  (`/Engine/EditorBlueprintResources/ActorMacros.Switch Has Authority`
    (:`Authority`
      (if (`self.canPickUp`)
        (bind _asmycharacter_c (cast `/Game/Blueprints/MyCharacter` OtherActor))
        (bind _canpickup (`/Game/Blueprints/MyCharacter.CanPickUpFlag` _asmycharacter_c))
        (if _canpickup
          (set `self.canPickUp` false)
          (`self.AttachRootComponentToActor` _asmycharacter_c "None" "SnapToTarget")
          (set `/Game/Blueprints/MyCharacter.carryingFlag` self _asmycharacter_c))))))

(fn `Reset`
  (`/Engine/EditorBlueprintResources/ActorMacros.Switch Has Authority`
    (:`Authority`
      (set `self.canPickUp` true)
      (bind _asmycharacter_c (cast `/Game/Blueprints/MyCharacter` (`ActorComponent.GetOwner` (`SceneComponent.GetAttachParent` (`self.K2_GetRootComponent`)))))
      (`/Game/Blueprints/MyCharacter.resetFlag` _asmycharacter_c)
      (`self.DetachRootComponentFromParent` true)
      (`self.K2_SetActorLocation` (`self.baseLocation`)))))

(fn `UserConstructionScript`
  (set `self.baseLocation` (`self.K2_GetActorLocation`)))