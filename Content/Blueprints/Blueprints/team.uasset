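; Team Blueprint that tracks a score and a count of frozen players, apparently for a freeze-tag style round game.
; Events wrap functions that raise or lower the frozen count, add a point for a round win, or check the win condition, all gated to run only with authority.
; The win check only prints the team's class name, showing it on screen when the frozen count equals the player list length, and does not award the win itself.
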(event `Increase Freeze Count Event`
  (`/Engine/EditorBlueprintResources/ActorMacros.Switch Has Authority`
    (:`Authority`
      (`self.increaseFreezeCount`))))

(event `Win Round Event`
  (`/Engine/EditorBlueprintResources/ActorMacros.Switch Has Authority`
    (:`Authority`
      (`self.winRound`))))

(event `Check Win Condition Event`
  (`/Engine/EditorBlueprintResources/ActorMacros.Switch Has Authority`
    (:`Authority`
      (`self.checkWinCondition`))))

(event `Decrease Freeze Condition Event`
  (`/Engine/EditorBlueprintResources/ActorMacros.Switch Has Authority`
    (:`Authority`
      (`self.decreaseFreezeCount`))))

(fn `checkWinCondition`
  (`KismetSystemLibrary.PrintString` (`KismetSystemLibrary.GetClassDisplayName` "Team_C") (== (`KismetArrayLibrary.Array_Length` (`self.listOfPlayers`)) (`self.frozenPeople`))))

(fn `decreaseFreezeCount`
  (set `self.frozenPeople` (- (`self.frozenPeople`) 1)))

(fn `increaseFreezeCount`
  (set `self.frozenPeople` (+ (`self.frozenPeople`) 1)))

(fn `UserConstructionScript`)

(fn `winRound`
  (set `self.Score` (+ (`self.Score`) 1)))