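; Game mode for a two-team flag game, Bruins versus Trojans, that assigns joining players to teams and spawns their characters.
; On the first authoritative PostLogin it spawns both Team actors, sorts PlayerStarts by tag and links flags and base areas by TeamIndex.
; Each login gets a Player actor on alternating teams.
; Once both teams have two players, characters spawn at team points and are possessed; the older SpawnTeam function is never called.
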(event `self.K2_PostLogin`
  (params (NewPlayer :type "PlayerController Object Reference"))
  (bind _returnvalue (`self.GetTransform`))
  (`/Engine/EditorBlueprintResources/ActorMacros.Switch Has Authority`
    (:`Authority`
      ;[1 1 1] spawn team actors
      (if (`self.Help`)
        (bind _returnvalue_2 (`|SpawnActorFromClass` "/Game/Blueprints/Blueprints/team.Team_C" _returnvalue true (`self.playerA`)))
        (set `self.teamA` _returnvalue_2)
        (set `/Game/Blueprints/Blueprints/team.Name` "Bruins" _returnvalue_2)
        (bind _returnvalue_3 (`|SpawnActorFromClass` "/Game/Blueprints/Blueprints/team.Team_C" _returnvalue true (`self.playerB`)))
        (set `self.teamB` _returnvalue_3)
        (set `/Game/Blueprints/Blueprints/team.Name` "Trojans" _returnvalue_3)
        (`self.setSpawnPoints`)
        ;[1 1 1] set flag team
        (bind _outactors (`GameplayStatics.GetAllActorsOfClass` "/Game/Blueprints/Flag.Flag_C"))
        (for _array_element _outactors
          (bind _asflag_c (cast `/Game/Blueprints/Flag` _array_element))
          (if (== (`/Game/Blueprints/Flag.TeamIndex` _asflag_c) 0)
            (set `/Game/Blueprints/Flag.Team` (`self.teamA`) _asflag_c)
            (else
              (set `/Game/Blueprints/Flag.Team` (`self.teamB`) _asflag_c))))
        ;[1 1 1] set base area teams
        (bind _outactors_2 (`GameplayStatics.GetAllActorsOfClass` "/Game/Blueprints/BaseArea.BaseArea_C"))
        (for _array_element_2 _outactors_2
          (bind _asbasearea_c (cast `/Game/Blueprints/BaseArea` _array_element_2))
          (if (== (`/Game/Blueprints/BaseArea.TeamIndex` _asbasearea_c) 0)
            (set `/Game/Blueprints/BaseArea.Team` (`self.teamA`) _asbasearea_c)
            (else
              (set `/Game/Blueprints/BaseArea.Team` (`self.teamB`) _asbasearea_c))))
        (set `self.Help` false))
      (`/Engine/EditorBlueprintResources/StandardMacros.CompareInt` (`self.currentTeam`)
        (:`>`
          (`self.placeOnTeamB` NewPlayer)
          (set `self.currentTeam` 0))
        (:`==`
          (`self.placeOnTeamA` NewPlayer)
          (set `self.currentTeam` 1)))
      (if (and (== (`KismetArrayLibrary.Array_Length` (`self.playerA`)) 2) (== (`KismetArrayLibrary.Array_Length` (`self.playerB`)) 2))
        (`self.spawnTeamA`)
        (`self.spawnTeamB`)))))

(fn `placeOnTeamA`
  (params (NewParam :type "PlayerController Object Reference"))
  (bind _indexa (`self.indexA`))
  (bind _item (`KismetArrayLibrary.Array_Get` (`self.playerA`) _indexa))
  (bind _returnvalue (`|SpawnActorFromClass` "/Game/Blueprints/Blueprints/Player.Player_C" (`self.GetTransform`)))
  (`KismetArrayLibrary.Array_Add` (`self.playerA`) _returnvalue)
  (set `/Game/Blueprints/Blueprints/Player.playerCon` NewParam _item)
  (set `/Game/Blueprints/Blueprints/Player.teamName` "teamA" _item)
  (`KismetArrayLibrary.Array_Add` (`/Game/Blueprints/Blueprints/team.listOfPlayers` (`self.teamA`)) _item)
  (`KismetSystemLibrary.PrintString` (`KismetStringLibrary.Conv_IntToString` (`KismetArrayLibrary.Array_Length` (`/Game/Blueprints/Blueprints/team.listOfPlayers` (`self.teamA`)))))
  (set `self.indexA` (+ _indexa 1)))

(fn `placeOnTeamB`
  (params (NewParam :type "PlayerController Object Reference"))
  (bind _indexb (`self.indexB`))
  (bind _item (`KismetArrayLibrary.Array_Get` (`self.playerB`) _indexb))
  (bind _returnvalue (`|SpawnActorFromClass` "/Game/Blueprints/Blueprints/Player.Player_C" (`self.GetTransform`)))
  (`KismetArrayLibrary.Array_Add` (`self.playerB`) _returnvalue)
  (set `/Game/Blueprints/Blueprints/Player.playerCon` NewParam _item)
  (set `/Game/Blueprints/Blueprints/Player.teamName` "teamB" _item)
  (`KismetArrayLibrary.Array_Add` (`/Game/Blueprints/Blueprints/team.listOfPlayers` (`self.teamB`)) _item)
  (`KismetSystemLibrary.PrintString` (`/Game/Blueprints/Blueprints/Player.teamName` (`KismetArrayLibrary.Array_Get` (`self.playerB`) _indexb)) true true (struct :`R` 1.0 :`G` 0.253274 :`B` 0.349054 :`A` 1.0))
  (set `self.indexB` (+ _indexb 1)))

(fn `setSpawnPoints`
  (bind _outactors (`GameplayStatics.GetAllActorsOfClass` "/Script/Engine.PlayerStart"))
  (for _array_element _outactors
    (bind _asplayerstart (cast `PlayerStart` _array_element))
    (if (== (`KismetArrayLibrary.Array_Get` (`Actor.Tags` _array_element)) "teamA")
      (`KismetArrayLibrary.Array_Add` (`self.spawnPointsA`) _asplayerstart)
      (else
        (`KismetArrayLibrary.Array_Add` (`self.spawnPointsB`) _asplayerstart)))))

(fn `spawnTeam`
  (for _index (range 4)
    (bind _outactors (`GameplayStatics.GetAllActorsOfClass` "/Script/Engine.PlayerStart"))
    (bind _returnvalue (`|SpawnActorFromClass` "/Game/Blueprints/MyCharacter.MyCharacter_C" (`self.GetTransform` (`KismetArrayLibrary.Array_Get` _outactors _index))))
    (`/Engine/EditorBlueprintResources/StandardMacros.CompareInt` (`self.spawnNum`)
      (:`>`
        (`Controller.Possess` (`/Game/Blueprints/Blueprints/Player.playerCon` (`KismetArrayLibrary.Array_Get` (`self.playerB`) (`self.spawnB`))) _returnvalue)
        (set `self.spawnNum` 0)
        (set `self.spawnB` (+ (`self.spawnB`) 1)))
      (:`==`
        (`Controller.Possess` (`/Game/Blueprints/Blueprints/Player.playerCon` (`KismetArrayLibrary.Array_Get` (`self.playerA`) (`self.spawnA`))) _returnvalue)
        (set `self.spawnNum` 1)
        (set `self.spawnA` (+ (`self.spawnA`) 1))))))

(fn `spawnTeamA`
  (for _index (range (`KismetArrayLibrary.Array_Length` (`self.playerA`)))
    (bind _item (`KismetArrayLibrary.Array_Get` (`self.playerA`) _index))
    (bind _returnvalue (`|SpawnActorFromClass` "/Game/Blueprints/MyCharacter.MyCharacter_C" (`self.GetTransform` (`KismetArrayLibrary.Array_Get` (`self.spawnPointsA`) _index)) false (`self.teamA`) _item))
    (`Controller.Possess` (`/Game/Blueprints/Blueprints/Player.playerCon` _item) _returnvalue)))

(fn `spawnTeamB`
  (for _index (range (`KismetArrayLibrary.Array_Length` (`self.playerB`)))
    (bind _item (`KismetArrayLibrary.Array_Get` (`self.playerB`) _index))
    (bind _returnvalue (`|SpawnActorFromClass` "/Game/Blueprints/MyCharacter.MyCharacter_C" (`self.GetTransform` (`KismetArrayLibrary.Array_Get` (`self.spawnPointsB`) _index)) false (`self.teamB`) _item))
    (`Controller.Possess` (`/Game/Blueprints/Blueprints/Player.playerCon` _item) _returnvalue)))

(fn `UserConstructionScript`)