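; MenuGameMode is the game mode for a menu, opening a connection on BeginPlay and servicing it every frame.
; Tick passes the game mode and the most recently logged-in player controller to a Dispatch call.
; PostLogin counts players, stores the new controller, and fires onLoginSuccess through a "ke *" console command.
; The onLoginSuccess handler only prints a debug string.
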(event `self.ReceiveBeginPlay`
  (`KismetSystemLibrary.PrintString` "connect")
  (`SuperNetwork.Connect`))

(event `self.ReceiveTick`
  (params (DeltaSeconds :type "Float (single-precision)"))
  (`SuperNetwork.dispatch` self (`self.pc`)))

(event `onLoginSuccess`
  (`KismetSystemLibrary.PrintString` "blah"))

(event `self.K2_PostLogin`
  (params (NewPlayer :type "PlayerController Object Reference"))
  (set `self.playerInt` (+ (`self.playerInt`) 1))
  (`KismetSystemLibrary.ExecuteConsoleCommand` "ke * onLoginSuccess" NewPlayer)
  (set `self.pc` NewPlayer))

(fn `UserConstructionScript`)