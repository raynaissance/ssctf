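; Chargeable Blueprint that manages a Charge value capped at 100, which drains per use and refills over time.
; SetDefaults stores the per-use drain and per-second refill rates.
; Discharge subtracts the drain, clamps at zero and starts Recharge.
; Recharge re-calls itself through a one-second Delay, adding charge via AddCharge until full, with debug prints reporting progress.
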(event Custom|recharge
  (if (< (Variables|Default|Getcharge) 100)
    (Utilities|FlowControl|Delay 1.0)
    (CallFunction|AddCharge)
    (CallFunction|Recharge)
    (else
      (Development|PrintString "DONE"))))

(fn ConstructionScript)

(fn Discharge
  (Math|Integer|CompareInt (|x-y (Variables|Default|Getcharge) (Variables|Default|GetdischargeUnits)) 0
    (:>
      (Variables|Default|Setcharge (|x-y (Variables|Default|Getcharge) (Variables|Default|GetdischargeUnits)) :!label _label))
    (:==
      (goto _label))
    (:<
      (Variables|Default|Setcharge 0)))
  (Development|PrintString (Utilities|String|ToString(Integer) (Variables|Default|Getcharge)))
  (CallFunction|Recharge))

(fn SetDefaults
  (params (dischargeUnitsPerUse :type Integer) (rechargeUnitsPerSec :type Integer))
  (Variables|Default|SetrechargePerSec rechargeUnitsPerSec)
  (Variables|Default|SetdischargeUnits dischargeUnitsPerUse)
  (Development|PrintString "Recharge Initialized"))

(fn AddCharge
  (Math|Integer|CompareInt (+ (Variables|Default|Getcharge) (Variables|Default|GetrechargePerSec)) 100
    (:>
      (Variables|Default|Setcharge 100))
    (:==
      (Variables|Default|Setcharge (+ (Variables|Default|Getcharge) (Variables|Default|GetrechargePerSec)) :!label _label)
      (Development|PrintString (Utilities|String|ToString(Integer) (+ (Variables|Default|Getcharge) (Variables|Default|GetrechargePerSec)))))
    (:<
      (goto _label))))