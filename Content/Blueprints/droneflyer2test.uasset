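; A test drone flyer actor that wanders between preset destination points.
; On BeginPlay a timeline lerps it from its start location to the current destination without sweeping.
; When the timeline finishes, it records its position, picks a random entry from the first five in the Destinations array, rerolling if it matches the current spot, and replays the timeline.
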(event `self.ReceiveBeginPlay`
  (set `self.StartPoint` (`self.K2_GetActorLocation`))
  (bind (_direction _percent) (`Timeline|Timeline_0` :!label _label)
    (:`Update`
      (`self.K2_SetActorLocation` (`KismetMathLibrary.VLerp` (`self.StartPoint`) (`self.Destination`) _percent)))
    (:`Finished`
      (set `self.StartPoint` (`self.K2_GetActorLocation`))
      (`self.setDestination` :!label _label_2)
      (if (== (`self.StartPoint`) (`self.Destination`))
        (goto _label_2)
        (else
          (goto _label :!via `PlayFromStart`))))))

(fn `setDestination`
  (set `self.Destination` (`KismetArrayLibrary.Array_Get` (`self.destinations`) (`KismetMathLibrary.RandomIntegerInRange` 0 4))))

(fn `UserConstructionScript`)