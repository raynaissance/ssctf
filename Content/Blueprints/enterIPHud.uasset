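; HUD Blueprint for a multiplayer main menu with IP entry, plus a lobby screen where the server gets a Start button.
; DrawHUD renders the screen selected by MainMenuActive and LobbyActive, using DrawButton with pressed-state textures.
; Number, period and delete keys edit the IP string through BuildHostString and DeleteStringChar.
; Hit box clicks set pressed states, and releases issue travel console commands to join, host a listen lobby or start the map.
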(event `self.ReceiveDrawHUD`
  (params (SizeX :type Integer) (SizeY :type Integer))
  (bind _buttontexture (`self.ButtonTexture`))
  (bind (_x _y) (`KismetMathLibrary.BreakVector2D` (`self.ScreenDimensions`)))
  (bind (_x_2 _y_2) (`KismetMathLibrary.BreakVector2D` (`self.ScreenDimensions`)))
  (set `self.ButtonSIze` (`KismetMathLibrary.MakeVector2D` (`KismetMathLibrary.Conv_IntToDouble` (`Texture2D.Blueprint_GetSizeX` _buttontexture)) (`KismetMathLibrary.Conv_IntToDouble` (`Texture2D.Blueprint_GetSizeY` _buttontexture))))
  (set `self.ScreenDimensions` (`KismetMathLibrary.MakeVector2D` (`KismetMathLibrary.Conv_IntToDouble` SizeX) (`KismetMathLibrary.Conv_IntToDouble` SizeY)))
  (if (`self.MainMenuActive`)
    ;[1 1 1] draw main menu
    (`self.DrawMaterialSimple` "/Game/HUD/Blueprints/menu2_Mat.menu2_Mat" 0.0 0.0 _x _y)
    (`self.DrawRect` (`self.TextBackgroundColor`) 400.0 350.0 400.0 50.0)
    (`self.DrawText` (`self.ipString`) (struct :`R` 0.28 :`G` 1.0 :`B` 0.467397 :`A` 1.0) 400.0 350.0 "/Game/HUD/Blueprints/myfont.myfont")
    (`self.DrawButton` (`KismetMathLibrary.MakeVector2D` 10.0 200.0) (`self.ButtonSIze`) "Play" (select `bool` (`self.PlayButtonPressed`) :`false` (`self.ButtonTexture`) :`true` (`self.ButtonTexturePressed`) :!type "Texture Object Reference") (`self.TextColor`))
    (`self.DrawButton` (`KismetMathLibrary.MakeVector2D` 10.0 300.0) (`self.ButtonSIze`) "Host" (select `bool` (`self.HostButtonPressed`) :`false` (`self.ButtonTexture`) :`true` (`self.ButtonTexturePressed`) :!type "Texture Object Reference") (`self.TextColor`))
    (if (`KismetSystemLibrary.IsServer`)
      (`KismetSystemLibrary.PrintString` "server?")
      (else
        (`KismetSystemLibrary.PrintString` "really not the server")))
    (elif (`self.LobbyActive`)
      ;[1 1 1] draw Lobby
      (`self.DrawMaterialSimple` "/Game/HUD/Blueprints/menu2_Mat.menu2_Mat" 0.0 0.0 _x_2 _y_2)
      (if (`KismetSystemLibrary.IsServer`)
        (`KismetSystemLibrary.PrintString` "I am the server")
        (`self.DrawButton` (`KismetMathLibrary.MakeVector2D` 10.0 300.0) (`self.ButtonSIze`) "Start" (select `bool` (`self.StartButtonPressed`) :`false` (`self.ButtonTexture`) :`true` (`self.ButtonTexturePressed`) :!type "Texture Object Reference") (`self.TextColor`))
        (else
          (`KismetSystemLibrary.PrintString` "waiting for game to start" true true (struct :`R` 0.25411 :`G` 1.0 :`B` 0.1 :`A` 1.0)))))))

(event `self.ReceiveHitBoxClick`
  (params (BoxName :type Name))
  (switch `name` BoxName
    (:`Play`
      (`KismetSystemLibrary.PrintString` "play")
      (set `self.PlayButtonPressed` true))
    (:`Start`
      (set `self.StartButtonPressed` true))
    (:`Host`
      (set `self.HostButtonPressed` true))))

(event `self.ReceiveHitBoxRelease`
  (params (BoxName :type Name))
  (switch `name` BoxName
    (:`Start`
      (set `self.LobbyActive` false)
      (set `self.MainMenuActive` false)
      (`KismetSystemLibrary.ExecuteConsoleCommand` (`KismetStringLibrary.Concat_StrStr` "ServerTravel " "Example_Map")))
    (:`Play`
      (`KismetSystemLibrary.PrintString` "play2")
      (`KismetSystemLibrary.ExecuteConsoleCommand` (`KismetStringLibrary.Concat_StrStr` "Travel " (`self.ipString`))))
    (:`Host`
      (`KismetSystemLibrary.ExecuteConsoleCommand` "Travel Lobby?Listen"))))

(event `Key|LeftMouseButton`
  (:`Released`
    (set `self.PlayButtonPressed` false)
    (set `self.StartButtonPressed` false)
    (set `self.HostButtonPressed` false)))

(event `Key|Three`
  ;[1 1 1] Key input
  (:`Pressed`
    (`self.BuildHostString` "3")))

(event `Key|One`
  ;[1 1 1] Key input
  (:`Pressed`
    (`self.BuildHostString` "1")))

(event `Key|Four`
  ;[1 1 1] Key input
  (:`Pressed`
    (`self.BuildHostString` "4")))

(event `Key|Two`
  ;[1 1 1] Key input
  (:`Pressed`
    (`self.BuildHostString` "2")))

(event `Key|Five`
  ;[1 1 1] Key input
  (:`Pressed`
    (`self.BuildHostString` "5")))

(event `Key|Seven`
  ;[1 1 1] Key input
  (:`Pressed`
    (`self.BuildHostString` "7")))

(event `Key|Six`
  ;[1 1 1] Key input
  (:`Pressed`
    (`self.BuildHostString` "6")))

(event `Key|Eight`
  ;[1 1 1] Key input
  (:`Pressed`
    (`self.BuildHostString` "8")))

(event `Key|Nine`
  ;[1 1 1] Key input
  (:`Pressed`
    (`self.BuildHostString` "9")))

(event `Key|Zero`
  ;[1 1 1] Key input
  (:`Pressed`
    (`self.BuildHostString` "0")))

(event `Key|Period`
  ;[1 1 1] Key input
  (:`Pressed`
    (`self.BuildHostString` ".")))

(event `Key|BackSpace`
  ;[1 1 1] Key input
  (:`Pressed`
    (`self.DeleteStringChar` :!label _label)))

(event `Key|Delete`
  ;[1 1 1] Key input
  (:`Pressed`
    (goto _label)))

(fn `UserConstructionScript`)